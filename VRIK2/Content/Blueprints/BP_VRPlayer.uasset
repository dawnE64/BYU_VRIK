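; VR player Blueprint that enables floor-origin stereo tracking and makes a detached skeletal body follow the headset.
; Each tick, camera movement or yaw change beyond thresholds sets a new body target behind and below the camera, plus a movement speed.
; Otherwise the body lerps toward that target at that speed, while its height updates every tick for IK.
; GetDirection's angle math is left unconnected.
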(event EventBeginPlay
  (Development|ExecuteConsoleCommand "stereo on" 0)
  (Class|HeadMountedDisplayFunctionLibrary|SetTrackingOrigin "Floor"))

(event EventTick
  (params (DeltaSeconds :type Float%20%28single-precision%29))
  (CallFunction|CalculateMovement))

(fn ConstructionScript
  (Transformation|DetachFromComponent (Variables|Default|GetSkeletalMesh) "KeepRelative" "KeepRelative" "KeepRelative" true))

(fn CalculateMovement
  (bind (_location _rotation) (CallFunction|GetBodyOffset))
  (bind _camera (Variables|Default|GetCamera))
  (bind _returnvalue (Transformation|GetWorldTransform _camera))
  (bind _output_get (LocalVariables|SetCurrentCameraPosition (Math|Transform|MakeTransform (Math|Vector|MakeVector (.x (.location _returnvalue)) (.y (.location _returnvalue)) 0.0) (Math|Rotator|MakeRotator 0.0 0.0 (.yaw (.rotation _returnvalue))) "1.000000,1.000000,1.000000")))
  (LocalVariables|SetDistanceMoved (CallFunction|GetDistanceMoved (.x (.location _output_get)) (.y (.location _output_get))))
  (LocalVariables|SetDistanceRotated (CallFunction|GetDistanceRotated (.rotation _output_get)))
  (Utilities|FlowControl|Sequence
    (:then_0
      ;[1 1 1] Move the body if a threshhold is met. Set new position. Otherwise lerp to position.
      (if (or (> (LocalVariables|GetDistanceMoved) (Variables|Default|GetMovementThreshold)) (> (LocalVariables|GetDistanceRotated) (Variables|Default|GetRotationThreshold)))
        ;;[0.3501 1 0.2964] Movement thresholds met
        (Variables|Default|SetBodyTargetPosition (Math|Transform|MakeTransform _location _rotation "1.000000,1.000000,1.000000"))
        (Variables|Default|SetMovementDirection (Utilities|GetDirection (LocalVariables|GetCurrentCameraPosition)))
        (Variables|Default|SetLastCameraPosition (LocalVariables|GetCurrentCameraPosition))
        (Variables|Default|SetMovementSpeed (/ (/ (+ (LocalVariables|GetDistanceMoved) (LocalVariables|GetDistanceRotated)) 2e+03) (Utilities|Time|GetWorldDeltaSeconds)))
        (elif (== (Variables|Default|GetBodyCurrentPosition) (Variables|Default|GetBodyTargetPosition))
          (Variables|Default|SetMovementSpeed 0.0)
          (Variables|Default|SetMovementDirection 0.0)
          (Variables|Default|SetAlpha 0.0)
          (else
            (Variables|Default|SetAlpha (Math|Interpolation|FInterptoConstant (Variables|Default|GetAlpha) 1.0 (Utilities|Time|GetWorldDeltaSeconds) (Variables|Default|GetMovementSpeed)))
            (bind _output_get_2 (Variables|Default|SetBodyCurrentPosition (Math|Transform|Lerp(Transform) (Variables|Default|GetBodyCurrentPosition) (Variables|Default|GetBodyTargetPosition) (Variables|Default|GetAlpha))))
            (Transformation|SetWorldLocationAndRotation (Variables|Default|GetSkeletalMesh) (.location _output_get_2) (.rotation _output_get_2) false false)))))
    (:then_1
      ;;[1 0.01848 0] Always set Z for IK (later would want to check for ground height)
      (Transformation|SetWorldLocationAndRotation (Variables|Default|GetSkeletalMesh) (Math|Vector|MakeVector (.x (.location (Variables|Default|GetBodyCurrentPosition))) (.y (.location (Variables|Default|GetBodyCurrentPosition))) (.z (.Location (CallFunction|GetBodyOffset)))) (.rotation (Variables|Default|GetBodyCurrentPosition)) false false))))

(fn GetDistanceMoved
  (params (CurrentX :type Float%20%28double-precision%29) (CurrentY :type Float%20%28double-precision%29))
  (bind _lastcameraposition (Variables|Default|GetLastCameraPosition))
  (return (Math|Vector|Distance(Vector) (Math|Vector|MakeVector CurrentX CurrentY 0.0) (Math|Vector|MakeVector (.x (.location _lastcameraposition)) (.y (.location _lastcameraposition)) 0.0))))

(fn GetDistanceRotated
  (params (CurrentRotation :type Rotator))
  (return (Math|Float|Absolute(Float) (- (.yaw CurrentRotation) (.yaw (.rotation (Variables|Default|GetLastCameraPosition)))))))

(fn GetBodyRotationfromHMD
  (return (Math|Rotator|MakeRotator 0.0 0.0 (- (.yaw (.rotation (Transformation|GetWorldTransform (Variables|Default|GetCamera)))) 9e+01))))

(fn GetBodyOffset
  (bind _camera (Variables|Default|GetCamera))
  (bind _returnvalue (Transformation|GetWorldTransform _camera))
  (bind _returnvalue_2 (- (.yaw (.rotation _returnvalue)) 9e+01))
  (bind _returnvalue_3 (Math|Rotator|MakeRotator 0.0 0.0 _returnvalue_2))
  (bind _returnvalue_4 (Math|Vector|GetRightVector _returnvalue_3))
  (bind _returnvalue_5 (* _returnvalue_4 -20))
  (bind _returnvalue_6 (+ (.location _returnvalue) _returnvalue_5))
  (return (Math|Vector|MakeVector (.x _returnvalue_6) (.y _returnvalue_6) (- (.z _returnvalue_6) (Variables|Default|GetPlayerHeight))) _returnvalue_3))