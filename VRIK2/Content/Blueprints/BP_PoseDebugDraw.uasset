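; Debug pose player that loops through numbered pose strings in the first registered string table, advancing every ANIMSPEED seconds.
; SetAllPoseRotations parses each string into floats scaled by VALSCALER and maps consecutive triples to rotators for 22 named body joints.
; GetAllRotations exposes those rotators to other code.
; The sphere-drawing path is an uncalled leftover, noted as unneeded because the values are rotations rather than locations.
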(event EventBeginPlay
  (CallFunction|SetAllPoseRotations (Class|KismetStringTableLibrary|GetTableEntrySourceString (Utilities|Array|Get(acopy) (Class|KismetStringTableLibrary|GetRegisteredStringTables)) (Utilities|String|ToString(Integer) (Variables|Default|GetStringKey))) :!label _label)
  (Utilities|FlowControl|Delay (Variables|Default|GetANIM_SPEED))
  (bind _result (Math|Integer|IncrementInt (Variables|Default|GetStringKey))
    (:%20%20
      (if (<= _result 52)
        (goto _label)
        (else
          (Variables|Default|SetStringKey 1)
          (goto _label))))))

(fn ConstructionScript)

(fn DrawDebugPose
  (params (PoseString :type String))
  (bind _output_get (Variables|Default|SetFloatArray (Utilities|String|ParseIntoArray PoseString " ")))
  (Variables|Default|SetNumValues (Utilities|Array|Length _output_get))
  (while (< (Variables|Default|GetIndex) (Variables|Default|GetNumValues))
    (Development|PrintString "BATCH")
    (bind (_x _y _z) (CallFunction|GetNextThreeFloats))
    (Depricated|DrawOneJoint (Math|Vector|MakeVector _x _y _z))))

(fn DrawOneJoint
  (params (Pose :type Vector))
  ;[1 0.01189 0] Turns out the values are not locations so this is uneeded
  (Rendering|Debug|DrawDebugSphere (Math|Vector|MakeVector (.x Pose) (.y Pose) (.z Pose)) 1e+01 12 "(R=1.000000,G=0.026817,B=0.000000,A=1.000000)" 2e+01 1.0))

(fn GetNextThreeFloats
  (bind _nextfloat (CallFunction|GetNextFloat))
  (bind _nextfloat_2 (CallFunction|GetNextFloat))
  (bind _nextfloat_3 (CallFunction|GetNextFloat))
  (return _nextfloat _nextfloat_2 _nextfloat_3))

(fn GetNextFloat
  (LocalVariables|SetToReturn (Math|Conversions|ToFloat(Integer) (Utilities|Array|Get(acopy) (Variables|Default|GetFloatArray) (Variables|Default|GetIndex))))
  (Math|Integer|IncrementInt (Variables|Default|GetIndex)
    (:%20%20
      (return (* (LocalVariables|GetToReturn) (Variables|Default|GetVAL_SCALER))))))

(fn SetAllPoseRotations
  (params (PoseString :type String))
  (Variables|Default|SetIndex 0)
  (Variables|Default|SetFloatArray (Utilities|String|ParseIntoArray PoseString " "))
  (while (<= (Variables|Default|GetIndex) 63)
    (bind (_x _y _z) (CallFunction|GetNextThreeFloats))
    (switch int (/ (- (Variables|Default|GetIndex) 1) 3)
      (:0
        (Variables|Default|SetPelvis (Math|Rotator|MakeRotator _x _y _z)))
      (:1
        (Variables|Default|SetLeftHip (Math|Rotator|MakeRotator _x _y _z)))
      (:2
        (Variables|Default|SetRightHip (Math|Rotator|MakeRotator _x _y _z)))
      (:3
        (Variables|Default|SetSpine1 (Math|Rotator|MakeRotator _x _y _z)))
      (:4
        (Variables|Default|SetLeft%20Knee (Math|Rotator|MakeRotator _x _y _z)))
      (:5
        (Variables|Default|SetRight%20Knee (Math|Rotator|MakeRotator _x _y _z)))
      (:6
        (Variables|Default|SetSpine%202 (Math|Rotator|MakeRotator _x _y _z)))
      (:7
        (Variables|Default|SetLeft%20Ankle (Math|Rotator|MakeRotator _x _y _z)))
      (:8
        (Variables|Default|SetRight%20Ankle (Math|Rotator|MakeRotator _x _y _z)))
      (:9
        (Variables|Default|SetSpine%203 (Math|Rotator|MakeRotator _x _y _z)))
      (:10
        (Variables|Default|SetLeft%20Foot (Math|Rotator|MakeRotator _x _y _z)))
      (:11
        (Variables|Default|SetRight%20Foot (Math|Rotator|MakeRotator _x _y _z)))
      (:12
        (Variables|Default|SetNeck (Math|Rotator|MakeRotator _x _y _z)))
      (:13
        (Variables|Default|SetLeft%20Collar (Math|Rotator|MakeRotator _x _y _z)))
      (:14
        (Variables|Default|SetRight%20Collar (Math|Rotator|MakeRotator _x _y _z)))
      (:15
        (Variables|Default|SetHead (Math|Rotator|MakeRotator _x _y _z)))
      (:16
        (Variables|Default|SetLeft%20Shoulder (Math|Rotator|MakeRotator _x _y _z)))
      (:17
        (Variables|Default|SetRight%20Shoulder (Math|Rotator|MakeRotator _x _y _z)))
      (:18
        (Variables|Default|SetLeft%20Elbow (Math|Rotator|MakeRotator _x _y _z)))
      (:19
        (Variables|Default|SetRight%20Elbow (Math|Rotator|MakeRotator _x _y _z)))
      (:20
        (Variables|Default|SetLeft%20Wrist (Math|Rotator|MakeRotator _x _y _z)))
      (:21
        (Variables|Default|SetRight%20Wrist (Math|Rotator|MakeRotator _x _y _z))))))

(fn GetAllRotations
  (return (Variables|Default|GetPelvis) (Variables|Default|GetLeftHip) (Variables|Default|GetRightHip) (Variables|Default|GetSpine1) (Variables|Default|GetLeft%20Knee) (Variables|Default|GetRight%20Knee) (Variables|Default|GetSpine%202) (Variables|Default|GetLeft%20Ankle) (Variables|Default|GetRight%20Ankle) (Variables|Default|GetSpine%203) (Variables|Default|GetLeft%20Foot) (Variables|Default|GetRight%20Foot) (Variables|Default|GetNeck) (Variables|Default|GetLeft%20Collar) (Variables|Default|GetRight%20Collar) (Variables|Default|GetHead) (Variables|Default|GetLeft%20Shoulder) (Variables|Default|GetRight%20Shoulder) (Variables|Default|GetLeft%20Elbow) (Variables|Default|GetRight%20Elbow) (Variables|Default|GetLeft%20Wrist) (Variables|Default|GetRight%20Wrist)))